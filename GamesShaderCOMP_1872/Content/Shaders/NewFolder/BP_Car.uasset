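; BP_Car is a Character-based pawn, named as a car, that the player drives with axis inputs.
; Forward and sideways axes add movement along the capsule's forward and right vectors, while the turn axis adds controller yaw.
; A Speed event sets the movement component's max walk speed and caches it in a variable that also scales forward input, but not sideways input.
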(event Custom|Speed
  (params (Speed :type Float%20%28single-precision%29))
  (bind _output_get (Variables|/Script/Engine.CharacterMovementComponent|SetMaxWalkSpeed (Variables|Character|GetCharacterMovement) Speed))
  (bind _output_get_2 (Variables|Default|SetSpeeeed _output_get)))

(event Input|AxisEvents|InputAxisMoveFoward
  (params (AxisValue :type Float%20%28single-precision%29))
  (Pawn|Input|AddMovementInput (Math|Vector|GetForwardVector (Variables|Collision|GetCapsuleComponent)) (* (stale Custom|Speed _output_get_2) AxisValue) false))

(event Input|AxisEvents|InputAxisMovdeSides
  (params (AxisValue :type Float%20%28single-precision%29))
  (Pawn|Input|AddMovementInput (Math|Vector|GetRightVector (Variables|Collision|GetCapsuleComponent)) AxisValue false))

(event Input|AxisEvents|InputAxisTurn
  (params (AxisValue :type Float%20%28single-precision%29))
  (Pawn|Input|AddControllerYawInput AxisValue))

(fn ConstructionScript)