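; Pickup actor that swaps a target mesh's material when a BP_Car enters its sphere; despite the SpeedUp name, it changes no speed.
; On overlap, if not hidden, it prints debug text, hides itself and applies a random entry from Materials to TargetMesh.
; Chained delays unhide it shortly after, then later restore M_Basic_Wall on the mesh.
; An unconnected chain using a Test material never runs.
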(event OnComponentBeginOverlap(Sphere)
  (params (OverlappedComponent :type Primitive%20Component%20Object%20Reference) (OtherActor :type Actor%20Object%20Reference) (OtherComp :type Primitive%20Component%20Object%20Reference) (OtherBodyIndex :type Integer) (bFromSweep :type Boolean) (SweepResult :type Hit%20Result%20Structure%20%28by%20ref%29))
  (if (not (Variables|Rendering|GetbHidden))
    (Utilities|Casting|CastToBP_Car OtherActor)
    (Development|PrintText "Hello")
    (Rendering|SetActorHiddenInGame true)
    (Rendering|Material|SetMaterial (Variables|/Script/Engine.StaticMeshActor|GetStaticMeshComponent (Variables|Default|GetTargetMesh)) 0 (Utilities|Array|Get(acopy) (Variables|Default|GetMaterials) (Math|Random|RandomIntegerinRange 0 (- (Utilities|Array|Length (Variables|Default|GetMaterials)) 1))))
    (Utilities|FlowControl|Delay 1.0)
    (Rendering|SetActorHiddenInGame false)
    (Utilities|FlowControl|Delay 7.0)
    (Rendering|SetActorHiddenInGame false)
    (Rendering|Material|SetMaterial (Variables|/Script/Engine.StaticMeshActor|GetStaticMeshComponent (Variables|Default|GetTargetMesh)) 0 "/Game/StarterContent/Materials/M_Basic_Wall.M_Basic_Wall")))

(event EventBeginPlay)

(event Collision|EventActorBeginOverlap
  (params (OtherActor :type Actor%20Object%20Reference)))

(event EventTick
  (params (DeltaSeconds :type Float%20%28single-precision%29)))

(fn ConstructionScript)