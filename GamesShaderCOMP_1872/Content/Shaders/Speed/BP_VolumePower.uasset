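; BP_VolumePower is a pickup that briefly applies a screen-wide post-process effect when a BP_Car touches it.
; The sphere overlap hides the actor and sets VolumenPP to unbound, then after a timed delay shows the actor again and re-bounds the effect.
; The Hidden flag blocks retriggering while the effect is active; the final delay has nothing after it, and NewFunction is an empty stub.
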(event OnComponentBeginOverlap(Sphere)
  (params (OverlappedComponent :type Primitive%20Component%20Object%20Reference) (OtherActor :type Actor%20Object%20Reference) (OtherComp :type Primitive%20Component%20Object%20Reference) (OtherBodyIndex :type Integer) (bFromSweep :type Boolean) (SweepResult :type Hit%20Result%20Structure%20%28by%20ref%29))
  (if (not (Variables|Rendering|GetbHidden))
    (Utilities|Casting|CastToBP_Car OtherActor)
    (Development|PrintText "Valume")
    (Rendering|SetActorHiddenInGame true)
    (Variables|/Script/Engine.PostProcessVolume|SetbUnbound (Variables|Default|GetVolumenPP) true)
    (Utilities|FlowControl|Delay 3.0)
    (Rendering|SetActorHiddenInGame false)
    (Variables|/Script/Engine.PostProcessVolume|SetbUnbound (Variables|Default|GetVolumenPP) false)
    (Utilities|FlowControl|Delay 2.0)))

(event EventBeginPlay)

(event Collision|EventActorBeginOverlap
  (params (OtherActor :type Actor%20Object%20Reference)))

(event EventTick
  (params (DeltaSeconds :type Float%20%28single-precision%29)))

(fn ConstructionScript)

(fn NewFunction
  (params (self2 :type Post%20Process%20Volume%20Object%20Reference)))